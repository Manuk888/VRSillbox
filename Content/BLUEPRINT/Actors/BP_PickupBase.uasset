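; BP_PickupBase is a pickup actor whose static mesh can be gripped and dropped by an interactor.
; The construction script applies the Mesh variable to the component.
; Grip disables physics and attaches the mesh component, snapping and offsetting it by its "Grip" socket transform if present, otherwise keeping its world location and rotation.
; Drop re-enables physics and detaches the mesh.
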(event EventBeginPlay)

(event Collision|EventActorBeginOverlap
  (params (OtherActor :type Actor%20Object%20Reference)))

(event EventTick
  (params (DeltaSeconds :type Float%20%28single-precision%29)))

(event EventDrop
  (Physics|SetSimulatePhysics (Variables|Default|GetStaticMesh) true)
  (Transformation|DetachFromComponent (Variables|Default|GetStaticMesh) "KeepRelative" "KeepRelative" "KeepRelative" true))

(event EventGrip
  (params (interactor :type Sphere%20Component%20Object%20Reference))
  (bind _staticmesh (Variables|Default|GetStaticMesh))
  (bind _returnvalue (Transformation|GetSocketTransform _staticmesh "Grip" "RTS_Actor"))
  (Physics|SetSimulatePhysics (Variables|Default|GetStaticMesh) false)
  (if (Transformation|DoesSocketExist (Variables|Default|GetStaticMesh) "Grip")
    (Transformation|AttachComponentToComponent (Variables|Default|GetStaticMesh) interactor "None" "SnapToTarget" "SnapToTarget" "KeepRelative" true)
    (Transformation|AddRelativeLocation (Variables|Default|GetStaticMesh) (* (Transformation|GetWorldScale (Variables|Default|GetStaticMesh)) (.Location (Math|Transform|BreakTransform (Math|Transform|InvertTransform _returnvalue)))) false false)
    (Transformation|AddLocalRotation (Variables|Default|GetStaticMesh) (.Rotation (Math|Transform|BreakTransform _returnvalue)) false false)
    (else
      (Transformation|AttachComponentToComponent (Variables|Default|GetStaticMesh) interactor "None" "KeepWorld" "KeepWorld" "KeepRelative" true))))

(fn ConstructionScript
  (Components|StaticMesh|SetStaticMesh (Variables|Default|GetStaticMesh) (Variables|Default|GetMesh)))