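; BP_LampColor is a lamp actor whose spot light shifts between red and green based on a supplied value.
; Its UpdateValue event uses that value as the alpha of a linear color lerp from red to green and applies the result to the SpotLight.
; It runs no logic of its own on begin play, tick or construction, so color changes only when that event is called.
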(event EventBeginPlay
  (|CallParentFunction) ; This node is disabled and will not be called.\nDrag off pins to build functionality.
)

(event Collision|EventActorBeginOverlap
  (params (OtherActor :type Actor%20Object%20Reference))
  (|CallParentFunction OtherActor) ; This node is disabled and will not be called.\nDrag off pins to build functionality.
)

(event EventTick
  (params (DeltaSeconds :type Float%20%28single-precision%29))
  (|CallParentFunction DeltaSeconds) ; This node is disabled and will not be called.\nDrag off pins to build functionality.
)

(event EventUpdateValue
  (params (Value :type Float%20%28single-precision%29))
  (Rendering|Components|Light|SetLightColor (Variables|Default|GetSpotLight) (Math|Color|Lerp(LinearColor) (Class|KismetMathLibrary|LinearColorRed) (Class|KismetMathLibrary|LinearColorGreen) Value) true))

(fn ConstructionScript
  (|CallParentFunction))