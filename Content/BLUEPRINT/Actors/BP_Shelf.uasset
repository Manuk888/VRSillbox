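; BP_Shelf is a sliding shelf actor that is pulled open and pushed shut by gripping its handle.
; ShelHandle's grip and drop events set and clear the Interactor, while hover events swap the handle material as a highlight.
; Each Tick, a valid Interactor's world position is converted to actor space, offset by the handle's relative location, and its X, clamped between zero and MaxDistance, positions the Axis component.
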(event Custom|EventOnGrip
  (params (ParentComponent :type Sphere%20Component%20Object%20Reference))
  (Variables|Default|SetInteractor ParentComponent))

(event Custom|EventOnDrop
  (Variables|Default|SetInteractor 0))

(event Custom|EventOnHover
  (Rendering|Material|SetMaterial (Variables|Default|GetShel_handle) 0 "/Game/Materials/M_ColorPing_Inst.M_ColorPing_Inst"))

(event Custom|EventOnUnHover
  (Rendering|Material|SetMaterial (Variables|Default|GetShel_handle) 0 "/Game/StarterContent/Materials/M_Metal_Gold.M_Metal_Gold"))

(event EventBeginPlay
  (EventDispatchers|BindEventtoOnGrip (Variables|Default|GetShel_handle) (EventDispatchers|CreateEvent :!event Custom|EventOnGrip))
  (EventDispatchers|BindEventtoOnDrop (Variables|Default|GetShel_handle) (EventDispatchers|CreateEvent :!event Custom|EventOnDrop))
  (EventDispatchers|BindEventtoOnHover (Variables|Default|GetShel_handle) (EventDispatchers|CreateEvent :!event Custom|EventOnHover))
  (EventDispatchers|BindEventtoOnUnhover (Variables|Default|GetShel_handle) (EventDispatchers|CreateEvent :!event Custom|EventOnUnHover)))

(event Collision|EventActorBeginOverlap
  (params (OtherActor :type Actor%20Object%20Reference)))

(event EventTick
  (params (DeltaSeconds :type Float%20%28single-precision%29))
  (Variables|Default|GetInteractor
    (:then
      (Transformation|SetRelativeLocation (Variables|Default|GetAxis) (Math|Vector|MakeVector (Math|Float|Clamp(Float) (CallFunction|CalculateLocation) 0.0 (Variables|Default|GetmaxDistance)) 0.0 0.0) false false))
    (:else)))

(fn ConstructionScript)

(fn CalculateLocation
  (bind _interactor (Variables|Default|GetInteractor)
    (:then
      (return (.x (- (Math|Transform|InverseTransformLocation (Transformation|GetActorTransform) (Transformation|GetWorldLocation _interactor)) (Variables|/Script/Engine.SceneComponent|GetRelativeLocation (Variables|Default|GetShel_handle))))))
    (:else)))