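; BP_PickYachiki is a pickable physics prop whose static mesh comes from its Mesh variable.
; It binds to its grippable mesh component's grip and drop events, toggling physics as it attaches to the gripping component or detaches.
; An optional "Grip" socket snaps it into place using inverted-transform location and socket rotation; otherwise it keeps its world pose.
; GetStatus always returns one fixed enum value.
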(event Custom|OnGrip
  (params (ParentComponent :type Sphere%20Component%20Object%20Reference))
  (bind _bpc_cripablemesh (Variables|Default|GetBPC_CripableMesh))
  (bind _returnvalue (Transformation|GetSocketTransform _bpc_cripablemesh "Grip" "RTS_Actor"))
  (Physics|SetSimulatePhysics (Variables|Default|GetBPC_CripableMesh) false)
  (if (Transformation|DoesSocketExist (Variables|Default|GetBPC_CripableMesh) "Grip")
    (Transformation|AttachComponentToComponent (Variables|Default|GetBPC_CripableMesh) ParentComponent "None" "SnapToTarget" "SnapToTarget" "KeepRelative" true)
    (Transformation|AddRelativeLocation (Variables|Default|GetBPC_CripableMesh) (* (Transformation|GetWorldScale (Variables|Default|GetBPC_CripableMesh)) (.Location (Math|Transform|BreakTransform (Math|Transform|InvertTransform _returnvalue)))) false false)
    (Transformation|AddLocalRotation (Variables|Default|GetBPC_CripableMesh) (.Rotation (Math|Transform|BreakTransform _returnvalue)) false false)
    (else
      (Transformation|AttachComponentToComponent (Variables|Default|GetBPC_CripableMesh) ParentComponent "None" "KeepWorld" "KeepWorld" "KeepRelative" true))))

(event Custom|OnDrop
  (Physics|SetSimulatePhysics (Variables|Default|GetBPC_CripableMesh) true)
  (Transformation|DetachFromComponent (Variables|Default|GetBPC_CripableMesh) "KeepRelative" "KeepRelative" "KeepRelative" true))

(event EventBeginPlay
  (EventDispatchers|BindEventtoOnGrip (Variables|Default|GetBPC_CripableMesh) (EventDispatchers|CreateEvent :!event Custom|OnGrip))
  (EventDispatchers|BindEventtoOnDrop (Variables|Default|GetBPC_CripableMesh) (EventDispatchers|CreateEvent :!event Custom|OnDrop)))

(event Collision|EventActorBeginOverlap
  (params (OtherActor :type Actor%20Object%20Reference)))

(event EventTick
  (params (DeltaSeconds :type Float%20%28single-precision%29)))

(fn ConstructionScript
  (bind _bpc_cripablemesh (Variables|Default|GetBPC_CripableMesh))
  (Components|StaticMesh|SetStaticMesh _bpc_cripablemesh (Variables|Default|GetMesh))
  (Physics|SetSimulatePhysics _bpc_cripablemesh true))

(fn GetStatus
  (return "NewEnumerator0"))