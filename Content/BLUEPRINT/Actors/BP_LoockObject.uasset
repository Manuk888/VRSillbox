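; BP_LoockObject is a configurable inspectable prop with a static mesh and a text label.
; The construction script applies the mesh, uniform scale, and the label's text, size and color from variables.
; Loockat and LoockAway open and close a Tick gate that spins the mesh by a fixed per-frame step, independent of delta time.
; Interactbytrace toggles the label's visibility.
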(event EventBeginPlay)

(event Collision|EventActorBeginOverlap
  (params (OtherActor :type Actor%20Object%20Reference)))

(event EventTick
  (params (DeltaSeconds :type Float%20%28single-precision%29))
  (Utilities|FlowControl|Gate true
    (:Exit
      (Transformation|AddLocalRotation (Variables|Default|GetStaticMesh) "0,0.200000,0.000000" false false))))

(event EventInteractbytrace
  (params (Out%20Hit :type Hit%20Result%20Structure))
  (bind _textrender (Variables|Default|GetTextRender))
  (if (Variables|/Script/Engine.SceneComponent|GetbVisible (Variables|Default|GetTextRender))
    (Rendering|SetVisibility _textrender false false)
    (else
      (Rendering|SetVisibility _textrender true false))))

(event EventLoockat
  (Utilities|FlowControl|Gate true) ; enters at Open
)

(event EventLoockAway
  (Utilities|FlowControl|Gate true) ; enters at Close
)

(fn ConstructionScript
  (Components|StaticMesh|SetStaticMesh (Variables|Default|GetStaticMesh) (Variables|Default|GetMesh))
  (Transformation|SetWorldScale3D (Variables|Default|GetStaticMesh) (Math|Conversions|ToVector(Float) (Variables|Default|GetScale)))
  (Rendering|Components|TextRender|SetText (Variables|Default|GetTextRender) (Variables|Default|GetText))
  (Rendering|Components|TextRender|SetWorldSize (Variables|Default|GetTextRender) (Variables|Default|GetTexstSize))
  (Rendering|Components|TextRender|SetTextRenderColor (Variables|Default|GetTextRender) (Variables|Default|GetTextColor)))