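; BP_Button_2 is a labeled button actor that triggers a linked interactive actor when a trace hits its mesh.
; The construction script applies the configurable text and static mesh to the TextRender and ButtonMesh components.
; Its Interactbytrace event checks for a blocking hit on ButtonMesh, then sends InteractOSMessage to the InteractiveActor reference.
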(event EventBeginPlay)

(event Collision|EventActorBeginOverlap
  (params (OtherActor :type Actor%20Object%20Reference)))

(event EventTick
  (params (DeltaSeconds :type Float%20%28single-precision%29)))

(event EventInteractbytrace
  (params (Out%20Hit :type Hit%20Result%20Structure))
  (bind (_bblockinghit _binitialoverlap _time _distance _location _impactpoint _normal _impactnormal _physmat _hitactor _hitcomponent) (Collision|BreakHitResult Out%20Hit))
  (if _bblockinghit
    (if (== _hitcomponent (Variables|Default|GetButtonMesh))
      (Class|BPIButtonElectric|InteractOS(Message) (Variables|Default|GetInteractiveActor)))))

(fn ConstructionScript
  (Rendering|Components|TextRender|SetText (Variables|Default|GetTextRender) (Variables|Default|GetText))
  (Components|StaticMesh|SetStaticMesh (Variables|Default|GetButtonMesh) (Variables|Default|GetNew%20Mesh)))