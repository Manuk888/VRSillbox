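; BP_Vigruzka is a trigger actor, apparently an unloading zone, that plays an animation while at least two crate-type actors are inside its box.
; Overlap events add and remove actors implementing BPI_INteractYashik in an array, printing the added index for debugging.
; The referenced AnimC4D geometry cache plays forward when an addition leaves two or more entries, and in reverse when a removal leaves fewer than two.
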(event OnComponentBeginOverlap(Box)
  (params (OverlappedComponent :type Primitive%20Component%20Object%20Reference) (OtherActor :type Actor%20Object%20Reference) (OtherComp :type Primitive%20Component%20Object%20Reference) (OtherBodyIndex :type Integer) (bFromSweep :type Boolean) (SweepResult :type Hit%20Result%20Structure%20%28by%20ref%29))
  ;[1 1 1] Добавляем в массив элементы
  (if (Utilities|DoesObjectImplementInterface OtherActor "/Game/BLUEPRINT/Interfeces/BPI_INteractYashik.BPI_INteractYashik_C")
    (bind _returnvalue (Utilities|Array|Add (Variables|Default|GetComponenti%20Peresicaemie) OtherActor))
    (Development|PrintString (Utilities|String|ToString(Integer) _returnvalue) true true "(R=0.000000,G=0.660000,B=1.000000,A=1.000000)" 1e+01)
    (if (>= (Utilities|Array|LastIndex (Variables|Default|GetComponenti%20Peresicaemie)) 1)
      (Audio|Components|Audio|Play (Variables|/Script/GeometryCache.GeometryCacheActor|GetGeometryCacheComponent (Variables|Default|GetAnimC4D))))))

(event OnComponentEndOverlap(Box)
  (params (OverlappedComponent :type Primitive%20Component%20Object%20Reference) (OtherActor :type Actor%20Object%20Reference) (OtherComp :type Primitive%20Component%20Object%20Reference) (OtherBodyIndex :type Integer))
  (bind _componenti_peresicaemie (Variables|Default|GetComponenti%20Peresicaemie))
  ;[1 1 1] Удаляем из массива объект
  (if (Utilities|Array|IsValidIndex _componenti_peresicaemie (Utilities|Array|FindItem _componenti_peresicaemie OtherActor))
    (Utilities|Array|RemoveItem (Variables|Default|GetComponenti%20Peresicaemie) OtherActor)
    (if (< (Utilities|Array|LastIndex (Variables|Default|GetComponenti%20Peresicaemie)) 1)
      (Class|GeometryCacheComponent|PlayReversed (Variables|/Script/GeometryCache.GeometryCacheActor|GetGeometryCacheComponent (Variables|Default|GetAnimC4D))))))

(event EventBeginPlay)

(event Collision|EventActorBeginOverlap
  (params (OtherActor :type Actor%20Object%20Reference)))

(event EventTick
  (params (DeltaSeconds :type Float%20%28single-precision%29)))

(fn ConstructionScript)