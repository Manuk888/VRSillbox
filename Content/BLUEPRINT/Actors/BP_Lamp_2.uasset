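; Lamp actor whose spotlight can be toggled or explicitly switched on and off.
; InteractOS flips the SpotLight's visibility, while Turnon and TurnOff set it directly.
; GetStatus reports whether the light is visible, so the component's visibility serves as the lamp's on/off state without a separate variable.
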(event EventBeginPlay)

(event Collision|EventActorBeginOverlap
  (params (OtherActor :type Actor%20Object%20Reference)))

(event EventTick
  (params (DeltaSeconds :type Float%20%28single-precision%29)))

(event EventTurnon
  (Rendering|SetVisibility (Variables|Default|GetSpotLight) true false))

(event EventTurnOff
  (Rendering|SetVisibility (Variables|Default|GetSpotLight) false false))

(event EventInteractOS
  (bind _spotlight (Variables|Default|GetSpotLight))
  (Rendering|SetVisibility _spotlight (not (Variables|/Script/Engine.SceneComponent|GetbVisible _spotlight)) false))

(fn ConstructionScript)

(fn GetStatus
  (return (Rendering|IsVisible (Variables|Default|GetSpotLight))))