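; Button platform actor with left and right button components that operate referenced level actors through interface messages.
; BeginPlay binds two handlers, both on the right button component, and sets the left button's color and state from RightActor's status.
; The left handler sends an interact message to LeftActor when pressed.
; The right handler sends on/off messages to RightActor if it implements BPI_ElectricSwitchable, otherwise an interact message.
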(event Custom|ButtonRightPressed
  (params (ButtonState :type Boolean))
  (CallFunction|TryPressButton (Variables|Default|GetRightActor) ButtonState))

(event Custom|ButtonLeftPressed
  (params (ButtonState :type Boolean))
  (if ButtonState
    (Class|BPIButtonElectric|InteractOS(Message) (Variables|Default|GetLeftActor))))

(event EventBeginPlay
  (EventDispatchers|BindEventtoButtonPressed (Variables|Default|GetBPC_ButtonRight) (EventDispatchers|CreateEvent :!event Custom|ButtonRightPressed))
  (EventDispatchers|BindEventtoButtonPressed (Variables|Default|GetBPC_ButtonRight) (EventDispatchers|CreateEvent :!event Custom|ButtonLeftPressed))
  (CallFunction|UpdateButtonState (Variables|Default|GetBPC_ButtonLeft) (Variables|Default|GetRightActor)))

(event Collision|EventActorBeginOverlap
  (params (OtherActor :type Actor%20Object%20Reference)))

(event EventTick
  (params (DeltaSeconds :type Float%20%28single-precision%29)))

(fn ConstructionScript)

(fn TryPressButton
  (params (ReferenceActor :type Actor%20Object%20Reference) (State :type Boolean))
  (if (Utilities|IsValid ReferenceActor)
    (if (Utilities|DoesObjectImplementInterface ReferenceActor "/Game/BLUEPRINT/Interfeces/BPI_ElectricSwitchable.BPI_ElectricSwitchable_C")
      (if State
        (Class|BPIElectricSwitchable|Turnon(Message) ReferenceActor)
        (else
          (Class|BPIElectricSwitchable|TurnOff(Message) ReferenceActor)))
      (else
        (Class|BPIButtonElectric|InteractOS(Message) ReferenceActor)))))

(fn UpdateButtonState
  (params (BPC_Button :type BPC%20Button%20Object%20Reference) (ActorReference :type Actor%20Object%20Reference))
  (bind _enabled (Class|BPIElectricSwitchable|GetStatus(Message) ActorReference))
  (Default|SetButtonColor BPC_Button _enabled)
  (Variables|/Game/BLUEPRINT/Companents/BPC_Button.BPC_Button_C|SetButtonState BPC_Button _enabled))