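; BP_Lever is a grippable lever actor that either switches a linked InteractiveActor on and off or feeds it a continuous value.
; While gripped, Tick converts the interactor's local position to a clamped axis angle via atan2; on release it can interpolate back to its idle rotation.
; CheckLeverState broadcasts the normalized angle and uses DoOnce gates for toggle-zone crossings.
; UpdateAngleValue selects value messages or on/off messages with material swaps.
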(event Custom|EventOnGrip
  (params (ParentComponent :type Sphere%20Component%20Object%20Reference))
  (Variables|Default|SetInteractor ParentComponent)
  (Variables|States|SetIsEnabled true))

(event Custom|EventOnDrop
  (Variables|States|SetIsEnabled true)
  (Variables|States|SetLerping true)
  (Variables|Default|SetInteractor 0))

(event Custom|OnLeverActivate
  (params (LeverState :type Boolean))
  (bind _interactiveactor (Variables|Default|GetInteractiveActor))
  (if (not (Variables|MainSettings|GetUpdateAngleValue))
    (Rendering|Material|SetMaterial (Variables|Default|GetBPC_CripableMesh) 0 (select LeverState "/Game/Materials/M_ColorPing_Inst.M_ColorPing_Inst" "/Game/StarterContent/Materials/M_Wood_Floor_Walnut_Worn.M_Wood_Floor_Walnut_Worn"))
    (if LeverState
      (Class|BPIElectricSwitchable|Turnon(Message) _interactiveactor)
      (else
        (Class|BPIElectricSwitchable|TurnOff(Message) _interactiveactor)))))

(event Custom|OnUpdateLever
  (params (LeverAngle :type Float%20%28single-precision%29))
  (if (Variables|MainSettings|GetUpdateAngleValue)
    (Class|BPIElectricValue|UpdateValue(Message) (Variables|Default|GetInteractiveActor) LeverAngle)))

(event EventBeginPlay
  (EventDispatchers|BindEventtoOnGrip (Variables|Default|GetBPC_CripableMesh) (EventDispatchers|CreateEvent :!event Custom|EventOnGrip))
  (EventDispatchers|BindEventtoOnDrop (Variables|Default|GetBPC_CripableMesh) (EventDispatchers|CreateEvent :!event Custom|EventOnDrop))
  (EventDispatchers|BindEventtoActivateLever (EventDispatchers|CreateEvent :!event Custom|OnLeverActivate))
  (EventDispatchers|BindEventtoUpdateLever (EventDispatchers|CreateEvent :!event Custom|OnUpdateLever))
  (if (not (Variables|MainSettings|GetUpdateAngleValue))
    (bind _enabled (Class|BPIElectricSwitchable|GetStatus(Message) (Variables|Default|GetInteractiveActor)))
    (Rendering|Material|SetMaterial (Variables|Default|GetBPC_CripableMesh) 0 (select _enabled "/Game/Materials/M_ColorPing_Inst.M_ColorPing_Inst" "/Game/StarterContent/Materials/M_Wood_Floor_Walnut_Worn.M_Wood_Floor_Walnut_Worn"))
    (Transformation|SetRelativeRotation (Variables|Default|GetLevelAxis) (Math|Rotator|MakeRotator 0.0 0.0 (select _enabled (Variables|MainSettings|GetmaxAngle) (Variables|MainSettings|GetidleRotation))) false false)))

(event Collision|EventActorBeginOverlap
  (params (OtherActor :type Actor%20Object%20Reference)))

(event EventTick
  (params (DeltaSeconds :type Float%20%28single-precision%29))
  (Utilities|FlowControl|Sequence
    (:then_0
      (CallFunction|UpdateLevelRotation))
    (:then_1
      (CallFunction|LerpingLeverRotation))))

(fn ConstructionScript)

(fn UpdateLevelRotation
  (bind _returnvalue (Transformation|GetActorTransform))
  (bind _interactor (Variables|Default|GetInteractor))
  (bind _levelaxis (Variables|Default|GetLevelAxis))
  (bind _minangle (Variables|MainSettings|GetminAngle))
  (bind _maxangle (Variables|MainSettings|GetmaxAngle))
  (bind _returnvalue_2 (Transformation|GetWorldLocation _interactor))
  (bind _relativelocation (Variables|/Script/Engine.SceneComponent|GetRelativeLocation _levelaxis))
  (bind _returnvalue_3 (Math|Transform|InverseTransformLocation _returnvalue _returnvalue_2))
  (bind _returnvalue_4 (- _returnvalue_3 _relativelocation))
  (bind _returnvalue_5 (Class|KismetMathLibrary|DegAtan2 (.x _returnvalue_4) (.z _returnvalue_4)))
  (bind _returnvalue_6 (Math|Float|Clamp(Float) _returnvalue_5 _minangle _maxangle))
  (if (Utilities|IsValid (Variables|Default|GetInteractor))
    (Transformation|SetRelativeRotation (Variables|Default|GetLevelAxis) (Math|Rotator|MakeRotator 0.0 0.0 _returnvalue_6) false false)
    (CallFunction|CheckLeverState _returnvalue_6)))

(fn CheckLeverState
  (params (Angle :type Float%20%28single-precision%29))
  (Default|CallUpdateLever (Math|Float|MapRangeClamped Angle (Variables|MainSettings|GetminAngle) (Variables|MainSettings|GetmaxAngle) 0.0 1.0))
  (if (> Angle (- (Variables|MainSettings|GetmaxAngle) (Variables|MainSettings|GetToggleZoneHeight)))
    (Utilities|FlowControl|Sequence
      (:then_0
        (Utilities|FlowControl|DoOnce false :!label _label
          (:Completed
            (Variables|States|SetIsEnabled false)
            (Default|CallActivateLever true))))
      (:then_1
        (goto _label_2 Reset)))
    (else
      (Utilities|FlowControl|Sequence
        (:then_0
          (Utilities|FlowControl|DoOnce false :!label _label_2
            (:Completed
              (Default|CallActivateLever false))))
        (:then_1
          (goto _label Reset))))))

(fn LerpingLeverRotation
  (bind _returnvalue (Utilities|Time|GetWorldDeltaSeconds))
  (bind _idlerotation (Variables|MainSettings|GetidleRotation))
  (bind _returnspeed (Variables|MainSettings|GetReturnSpeed))
  (bind _levelaxis (Variables|Default|GetLevelAxis))
  (bind _relativerotation (Variables|/Script/Engine.SceneComponent|GetRelativeRotation _levelaxis))
  (bind _returnvalue_2 (Math|Interpolation|FInterpTo (.yaw _relativerotation) _idlerotation _returnvalue _returnspeed))
  (if (Math|Boolean|ANDBoolean (Variables|States|GetIsEnabled) (Variables|States|GetLerping) (Variables|MainSettings|GetReturnToStart))
    (if (> _returnvalue_2 (- (Variables|MainSettings|GetmaxAngle) (Variables|MainSettings|GetToggleZoneHeight)))
      (Variables|States|SetLerping false)
      (else
        (Transformation|SetRelativeRotation (Variables|Default|GetLevelAxis) (Math|Rotator|MakeRotator 0.0 0.0 _returnvalue_2) false false)
        (CallFunction|CheckLeverState _returnvalue_2)
        (if (== (Variables|MainSettings|GetidleRotation) (.yaw (Variables|/Script/Engine.SceneComponent|GetRelativeRotation (Variables|Default|GetLevelAxis))))
          (Variables|States|SetLerping false))))))