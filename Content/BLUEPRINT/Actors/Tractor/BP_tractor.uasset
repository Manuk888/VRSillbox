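; VR-drivable physics tractor with a bucket, which the BP_VRPawn player enters and exits via buttons that attach or detach the pawn.
; Four BP_Lever child actors supply left and right drive inputs plus target angles for bucket arm and bucket.
; Each tick applies tank-style forces at either side of the body, input-scaled drag, yaw damping and sideways-velocity cancellation.
; Bucket parts ease toward their target pitches through interpolation.
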(event Custom|Button_EnterPressed
  (params (ButtonState :type Boolean))
  ;[1 1 1] Вход в трактор
  (if ButtonState
    (bind _asbp_vrpawn (Utilities|Casting|CastToBP_VRPawn (Components|GetOwner (Variables|/Game/BLUEPRINT/Companents/BPC_Button.BPC_Button_C|GetFoucedComponent (Variables|Default|GetBPC_ButtonEnter)))))
    (bind _output_get (Variables|Default|SetVRPawn _asbp_vrpawn))
    (Variables|/Game/BLUEPRINT/Game/BP_VRPawn.BP_VRPawn_C|SetCanMove? _output_get false)
    (Class|HeadMountedDisplayFunctionLibrary|ResetOrientationandPosition 0.0 "OrientationAndPosition")
    (Transformation|AttachComponentToComponent (Variables|Default|GetVRPawn) (Variables|Default|GetArrow) "None" "SnapToTarget" "SnapToTarget" "KeepWorld" true)
    (Transformation|SetActorRelativeLocation (Variables|Default|GetVRPawn) "0, 0,40.000000")
    (Variables|/Game/BLUEPRINT/Game/BP_VRPawn.BP_VRPawn_C|SetUrovenGlaz (Variables|Default|GetVRPawn) "Eye")))

(event Custom|Button_ExitPressed
  (params (ButtonState :type Boolean))
  (bind _tractortires (Variables|Default|GetTractorTires))
  (bind _returnvalue (Transformation|GetWorldLocation _tractortires))
  (bind _returnvalue_2 (Math|Vector|GetRightVector _tractortires))
  (bind _returnvalue_3 (* _returnvalue_2 1.5e+02))
  (bind _returnvalue_4 (+ _returnvalue _returnvalue_3))
  ;[1 1 1] Exit Tractor
  (if ButtonState
    (Variables|/Game/BLUEPRINT/Game/BP_VRPawn.BP_VRPawn_C|SetCanMove? (Variables|Default|GetVRPawn) true)
    (Transformation|DetachFromActor (Variables|Default|GetVRPawn) "KeepRelative" "KeepRelative" "KeepRelative")
    (Transformation|AddWorldOffset (Variables|/Game/BLUEPRINT/Game/BP_VRPawn.BP_VRPawn_C|GetDefaultSceneRoot (Variables|Default|GetVRPawn)) (Math|Vector|MakeVector (.x _returnvalue_4) (.y _returnvalue_4) 0.0) false false)
    (Variables|/Game/BLUEPRINT/Game/BP_VRPawn.BP_VRPawn_C|SetUrovenGlaz (Variables|Default|GetVRPawn) "Eye")))

(event Custom|UpdateRightLaver
  (params (LeverAngle :type Float%20%28single-precision%29))
  ;[1 1 1] Set Input
  (Variables|Default|SetRightInput (Math|Float|MapRangeClamped LeverAngle 0.0 1.0 1.0 -1.0)))

(event Custom|UpdateLeftLaver
  (params (LeverAngle :type Float%20%28single-precision%29))
  ;[1 1 1] Set Input
  (Variables|Default|SetLeftInput (Math|Float|MapRangeClamped LeverAngle 0.0 1.0 1.0 -1.0)))

(event Custom|UpdateLeverAxis
  (params (LeverAngle :type Float%20%28single-precision%29))
  (Variables|Default|SetAxesBucketTargetAngle (* LeverAngle 7e+01)))

(event Custom|UpdateLaverBucket
  (params (LeverAngle :type Float%20%28single-precision%29))
  (Variables|Default|SetBucketTargetAngle (Math|Float|MapRangeClamped LeverAngle 0.0 1.0 -6e+01 6e+01)))

(event EventBeginPlay
  (EventDispatchers|BindEventtoButtonPressed (Variables|Default|GetBPC_ButtonEnter) (EventDispatchers|CreateEvent :!event Custom|Button_EnterPressed))
  (EventDispatchers|BindEventtoButtonPressed (Variables|Default|GetBPC_ButtonExite) (EventDispatchers|CreateEvent :!event Custom|Button_ExitPressed))
  (bind _asbp_lever (Utilities|Casting|CastToBP_Lever (Variables|/Script/Engine.ChildActorComponent|GetChildActor (Variables|Default|GetBP_LaverRight))))
  (EventDispatchers|BindEventtoUpdateLever _asbp_lever (EventDispatchers|CreateEvent :!event Custom|UpdateRightLaver))
  (bind _asbp_lever_2 (Utilities|Casting|CastToBP_Lever (Variables|/Script/Engine.ChildActorComponent|GetChildActor (Variables|Default|GetBP_LaverLeft))))
  (EventDispatchers|BindEventtoUpdateLever _asbp_lever_2 (EventDispatchers|CreateEvent :!event Custom|UpdateLeftLaver))
  (bind _asbp_lever_3 (Utilities|Casting|CastToBP_Lever (Variables|/Script/Engine.ChildActorComponent|GetChildActor (Variables|Default|GetBP_LaverBucketAxes))))
  (EventDispatchers|BindEventtoUpdateLever _asbp_lever_3 (EventDispatchers|CreateEvent :!event Custom|UpdateLeverAxis))
  (bind _asbp_lever_4 (Utilities|Casting|CastToBP_Lever (Variables|/Script/Engine.ChildActorComponent|GetChildActor (Variables|Default|GetBP_LaverBucket))))
  (EventDispatchers|BindEventtoUpdateLever _asbp_lever_4 (EventDispatchers|CreateEvent :!event Custom|UpdateLaverBucket)))

(event Collision|EventActorBeginOverlap
  (params (OtherActor :type Actor%20Object%20Reference)))

(event EventTick
  (params (DeltaSeconds :type Float%20%28single-precision%29))
  ;[1 1 1] tick
  (Utilities|FlowControl|Sequence
    (:then_0
      (CallFunction|UpdateForce))
    (:then_1
      (CallFunction|Damping))
    (:then_2
      (CallFunction|UpdateBucketAngle))))

(fn ConstructionScript)

(fn UpdateForce
  (if (or (> (Math|Float|Absolute(Float) (Variables|Default|GetLeftInput)) (Variables|Default|GetLeversDeadZone)) (> (Math|Float|Absolute(Float) (Variables|Default|GetRightInput)) (Variables|Default|GetLeversDeadZone)))
    (Utilities|FlowControl|Sequence
      (:then_0
        (Class|PrimitiveComponent|AddForceatLocation (Variables|Default|GetTractorTires) (* (Math|Vector|GetForwardVector (Variables|Default|GetTractorTires)) (* (Variables|Speed|GetPower) (Variables|Default|GetLeftInput) (Physics|GetMass (Variables|Default|GetTractorTires)))) (Math|Transform|TransformLocation (Transformation|GetWorldTransform (Variables|Default|GetTractorTires)) "0,-100.000000, 0") "None"))
      (:then_1
        (Class|PrimitiveComponent|AddForceatLocation (Variables|Default|GetTractorTires) (* (Math|Vector|GetForwardVector (Variables|Default|GetTractorTires)) (* (Variables|Speed|GetPower) (Variables|Default|GetRightInput) (Physics|GetMass (Variables|Default|GetTractorTires)))) (Math|Transform|TransformLocation (Transformation|GetWorldTransform (Variables|Default|GetTractorTires)) "0,100.000000, 0") "None")))))

(fn Damping
  (bind _tractortires (Variables|Default|GetTractorTires))
  (Physics|AddForce (Variables|Default|GetTractorTires) (* (Transformation|GetVelocity) (CallFunction|GetLinerStopingForce)) "None" false)
  (Class|PrimitiveComponent|SetPhysicsAngularVelocityinDegrees (Variables|Default|GetTractorTires) (Math|Vector|MakeVector 0.0 0.0 (CallFunction|GetAngularStopingForce)) false "None")
  (bind _returnvalue (Physics|GetPhysicsLinearVelocity _tractortires "None"))
  (Physics|SetPhysicsLinearVelocity (Variables|Default|GetTractorTires) (- _returnvalue (* (Math|Vector|GetRightVector (Variables|Default|GetTractorTires)) (Math|Vector|DotProduct _returnvalue (Math|Vector|GetRightVector _tractortires)))) false "None"))

(fn GetLinerStopingForce
  (return (Math|Float|MapRangeClamped (+ (Math|Float|Absolute(Float) (Variables|Default|GetLeftInput)) (Math|Float|Absolute(Float) (Variables|Default|GetRightInput))) 0.0 2.0 (Variables|Speed|GetOutZatuchanie%20Range%20A) (Variables|Speed|GetOutZatuchanie%20Range%20B))))

(fn GetAngularStopingForce
  (return (Math|Interpolation|FInterpTo (.z (Physics|GetPhysicsAngularVelocityinDegrees (Variables|Default|GetTractorTires) "None")) 0.0 (Utilities|Time|GetWorldDeltaSeconds) 5.0)))

(fn UpdateBucketAngle
  (Transformation|SetRelativeRotation (Variables|Default|Getsm_tracktor_bucketAxes) (Math|Rotator|MakeRotator 0.0 (Math|Interpolation|FInterpTo (.pitch (Variables|/Script/Engine.SceneComponent|GetRelativeRotation (Variables|Default|Getsm_tracktor_bucketAxes))) (Variables|Default|GetAxesBucketTargetAngle) (Utilities|Time|GetWorldDeltaSeconds) 1.0) 0.0) false false)
  (Transformation|SetRelativeRotation (Variables|Default|Getsm_tracktor_bucket) (Math|Rotator|MakeRotator 0.0 (Math|Interpolation|FInterpTo (.pitch (Variables|/Script/Engine.SceneComponent|GetRelativeRotation (Variables|Default|Getsm_tracktor_bucket))) (Variables|Default|GetBucketTargetAngle) (Utilities|Time|GetWorldDeltaSeconds) 1.0) 0.0) false false))