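; BPC_Hover is a hover-point component for BP_tractor that pushes the vehicle off the surface beneath it.
; Each tick it line-traces down its own up vector on Visibility up to HoverDistance, drawing debug.
; On a hit, it applies a spring-damper style force to the tractor's root at the component's location.
; DampingCoefficient scales both compression and rate terms, and PreviousDelta is never updated in this graph.
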(event EventBeginPlay
  (bind _asbp_tractor (Utilities|Casting|CastToBP_tractor (Components|GetOwner)))
  (Variables|Default|SetBP_Tractor _asbp_tractor))

(event EventTick
  (params (DeltaSeconds :type Float%20%28single-precision%29))
  (bind _returnvalue (Transformation|GetWorldLocation))
  (Variables|Default|GetBP_Tractor
    (:then
      (bind (_outhit _returnvalue_2) (Collision|LineTraceByChannel _returnvalue (- _returnvalue (* (Math|Vector|GetUpVector) (Variables|Default|GetHoverDistance))) "TraceTypeQuery1" false 0 "ForOneFrame"))
      (if _returnvalue_2
        (bind _output_get (Variables|Default|SethoverDelta (- (Variables|Default|GetHoverDistance) (.Distance (Collision|BreakHitResult _outhit)))))
        (Class|PrimitiveComponent|AddForceatLocation (.AsPrimitive%20Component (Utilities|Casting|CastToPrimitiveComponent (Variables|/Script/Engine.Actor|GetRootComponent (Variables|Default|GetBP_Tractor)))) (* (Math|Vector|GetUpVector) (+ (* (/ (- _output_get (Variables|Default|GetPreviousDelta)) (Utilities|Time|GetWorldDeltaSeconds)) (Variables|Default|GetDampingCoefficient)) (* _output_get (Variables|Default|GetDampingCoefficient)))) (Transformation|GetWorldLocation) "None")))
    (:else)))