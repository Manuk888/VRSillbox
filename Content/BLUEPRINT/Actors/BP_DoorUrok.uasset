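; Hinged door actor that an interactor can grip and swing by its handle, which changes material on hover.
; While gripped, Tick derives yaw from the interactor's local position around DoorAxes via atan2, minus the grab offset, clamped between angle limits.
; Entering the zone near MaxAngle stops the door following the grip.
; On release, if an angle check passes and ReturnToStart is set, yaw interpolates back to the idle rotation.
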(event Custom|EventOnGrip
  (params (ParentComponent :type Sphere%20Component%20Object%20Reference))
  (Variables|Default|Setinteractor ParentComponent)
  (Variables|Default|SetDoorStartOffset (- (CallFunction|CalculateAngle) (.yaw (Variables|/Script/Engine.SceneComponent|GetRelativeRotation (Variables|Default|GetDoorAxes)))))
  (Variables|States|SetIsEnabled true))

(event Custom|EventOnDrop
  (Variables|States|SetIsEnabled false)
  (Variables|Default|Setinteractor 0)
  (Variables|States|SetLerping (> (+ (Variables|MainSettings|GetClosingZoneOffset) (Math|Float|Absolute(Float) (Variables|Default|GetCurrentAngle))) (Math|Float|Absolute(Float) (Variables|MainSettings|GetidleRotetion)))))

(event Custom|EventOnHover
  (Rendering|Material|SetMaterial (Variables|Default|GetDoorHandle) 0 "/Game/Materials/M_ColorPing_Inst.M_ColorPing_Inst"))

(event Custom|EventOnUnHpver
  (Rendering|Material|SetMaterial (Variables|Default|GetDoorHandle) 0 "/Game/Materials/M_COLORGreen__Inst.M_COLORGreen__Inst"))

(event EventBeginPlay
  (EventDispatchers|BindEventtoOnGrip (Variables|Default|GetDoorHandle) (EventDispatchers|CreateEvent :!event Custom|EventOnGrip))
  (EventDispatchers|BindEventtoOnDrop (Variables|Default|GetDoorHandle) (EventDispatchers|CreateEvent :!event Custom|EventOnDrop))
  (EventDispatchers|BindEventtoOnHover (Variables|Default|GetDoorHandle) (EventDispatchers|CreateEvent :!event Custom|EventOnHover))
  (EventDispatchers|BindEventtoOnUnhover (Variables|Default|GetDoorHandle) (EventDispatchers|CreateEvent :!event Custom|EventOnUnHpver)))

(event Collision|EventActorBeginOverlap
  (params (OtherActor :type Actor%20Object%20Reference)))

(event EventTick
  (params (DeltaSeconds :type Float%20%28single-precision%29))
  (Utilities|FlowControl|Sequence
    (:then_0
      (CallFunction|UpdateDoorRotation))
    (:then_1
      (CallFunction|LerpingDoorRotation))))

(fn ConstructionScript)

(fn UpdateDoorRotation
  (bind _angle (CallFunction|CalculateAngle))
  (bind _doorstartoffset (Variables|Default|GetDoorStartOffset))
  (bind _minangle (Variables|MainSettings|GetMinAngle))
  (bind _maxangle (Variables|MainSettings|GetMaxAngle))
  (bind _returnvalue (- _angle _doorstartoffset))
  (bind _returnvalue_2 (Math|Float|Clamp(Float) _returnvalue _minangle _maxangle))
  (if (and (Utilities|IsValid (Variables|Default|Getinteractor)) (Variables|States|GetIsEnabled))
    (Variables|States|SetLerping false)
    (Transformation|SetRelativeRotation (Variables|Default|GetDoorAxes) (Math|Rotator|MakeRotator 0.0 0.0 _returnvalue_2) false false)
    (Variables|Default|SetCurrentAngle _returnvalue_2)
    (CallFunction|CheckDoorState _returnvalue_2)))

(fn CalculateAngle
  (bind _interactor (Variables|Default|Getinteractor)
    (:then
      (return (Class|KismetMathLibrary|DegAtan2 (.y (- (Math|Transform|InverseTransformLocation (Transformation|GetActorTransform) (Transformation|GetWorldLocation _interactor)) (Variables|/Script/Engine.SceneComponent|GetRelativeLocation (Variables|Default|GetDoorAxes)))) (.x (- (Math|Transform|InverseTransformLocation (Transformation|GetActorTransform) (Transformation|GetWorldLocation _interactor)) (Variables|/Script/Engine.SceneComponent|GetRelativeLocation (Variables|Default|GetDoorAxes)))))))
    (:else)))

(fn CheckDoorState
  (params (Angle :type Float%20%28single-precision%29))
  (if (> Angle (- (Variables|MainSettings|GetMaxAngle) (Variables|MainSettings|GetClosingZoneOffset)))
    (Utilities|FlowControl|DoOnce false :!label _label
      (:Completed
        (Variables|States|SetIsEnabled false)))
    (else
      (goto _label Reset))))

(fn LerpingDoorRotation
  (bind _returnvalue (Utilities|Time|GetWorldDeltaSeconds))
  (bind _idlerotetion (Variables|MainSettings|GetidleRotetion))
  (bind _returnspeed (Variables|MainSettings|GetReturnSpeed))
  (bind _dooraxes (Variables|Default|GetDoorAxes))
  (bind _relativerotation (Variables|/Script/Engine.SceneComponent|GetRelativeRotation _dooraxes))
  (bind _returnvalue_2 (Math|Interpolation|FInterpTo (.yaw _relativerotation) _idlerotetion _returnvalue _returnspeed))
  (if (and (Variables|States|GetLerping) (Variables|MainSettings|GetReturnToStart))
    (Transformation|SetRelativeRotation (Variables|Default|GetDoorAxes) (Math|Rotator|MakeRotator 0.0 0.0 _returnvalue_2) false false)
    (CallFunction|CheckDoorState _returnvalue_2)
    (if (== (Variables|MainSettings|GetidleRotetion) (.yaw (Variables|/Script/Engine.SceneComponent|GetRelativeRotation (Variables|Default|GetDoorAxes))))
      (Variables|States|SetLerping false))))