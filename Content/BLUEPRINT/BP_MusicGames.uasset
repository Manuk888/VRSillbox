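; Simon-style musical memory minigame actor: it plays a random button sequence that the player repeats through Interact.
; Components tagged MusicButton form the buttons, and a looping timer lights each note with its sound before enabling input.
; Presses match the hit component against the current note, giving material and sound feedback, with a timer restoring the color.
; Success regenerates a sequence one note longer, a mistake resets to one note, and TextRender shows the length.
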(event EventBeginPlay
  (Variables|Default|SetCurrentSequenceLoop 0)
  (CallFunction|CalculateNotes)
  (CallFunction|PlayNoteSequence))

(event Collision|EventActorBeginOverlap
  (params (OtherActor :type Actor%20Object%20Reference)))

(event EventTick
  (params (DeltaSeconds :type Float%20%28single-precision%29)))

(event EventInteract
  (params (Out%20Hit :type Hit%20Result%20Structure))
  (if (Variables|Default|GetIsinputMode)
    (bind (_success _correct _button_companent _buttonid) (CallFunction|TryPressButton (.HitComponent (Collision|BreakHitResult Out%20Hit))))
    (if _success
      (CallFunction|InteractButton _correct _buttonid))))

(fn ConstructionScript
  (CallFunction|BaseColor)
  (CallFunction|CollectButtons))

(fn BaseColor
  (Rendering|Material|SetMaterial (Variables|Default|Getmusic_games_Base) 0 "/Game/Materials/M_COLORElov_Inst1.M_COLORElov_Inst1"))

(fn CollectButtons
  (Utilities|Array|Clear (Variables|Default|GetButtons))
  (Variables|Default|SetButtons (Actor|GetComponentsbyTag "/Script/Engine.ActorComponent" "MusicButton"))
  (Variables|Default|SetButtons%20Cound (Utilities|Array|Length (Variables|Default|GetButtons))))

(fn CalculateNotes
  (Utilities|Array|Clear (Variables|Default|GetNotes))
  (LocalVariables|SetLocalMaxNotes (Variables|Default|GetCurrentSequenceLoop))
  (for _index (range 0 (LocalVariables|GetLocalMaxNotes))
    (Utilities|Array|Add (Variables|Default|GetNotes) (Math|Random|RandomInteger (Variables|Default|GetButtons%20Cound))))
  (Variables|Default|SetSizeOdSequence (Utilities|Array|Length (Variables|Default|GetNotes))))

(fn PlayNoteSequence
  (Variables|Default|SetIsinputMode false)
  (Variables|Default|SetNoteLoop 0)
  (bind _returnvalue (Utilities|Time|SetTimerbyFunctionName 0 "PlayNote" (Variables|Default|GetSpeedTime) true))
  (Variables|Default|SetPlayNoteTimer _returnvalue)
  (Rendering|Components|TextRender|SetText (Variables|Default|GetTextRender) (Utilities|Text|ToText(Integer) (Variables|Default|GetSizeOdSequence))))

(fn PlayNote
  (if (< (Variables|Default|GetNoteLoop) (Variables|Default|GetSizeOdSequence))
    (Variables|Default|SetCurrentNote (Utilities|Array|Get(acopy) (Variables|Default|GetNotes) (Variables|Default|GetNoteLoop)))
    (if (Variables|Default|GetIsTurnOn)
      (Variables|Default|SetIsTurnOn false)
      (bind _asstatic_mesh_component (Utilities|Casting|CastToStaticMeshComponent (Utilities|Array|Get(acopy) (Variables|Default|GetButtons) (Variables|Default|GetCurrentNote))))
      (Rendering|Material|SetMaterial _asstatic_mesh_component 0 "/Game/Materials/M_ColorPing_Inst.M_ColorPing_Inst")
      (Audio|PlaySoundatLocation (Utilities|Array|Get(acopy) (Variables|Default|GetSounds) (Variables|Default|GetCurrentNote)) (Transformation|GetWorldLocation (Variables|Default|Getmusic_games_Base)) "0, 0, 0" 1.0 1.0 0.0 0 0 0)
      (else
        (Variables|Default|SetIsTurnOn true)
        (bind _asstatic_mesh_component_2 (Utilities|Casting|CastToStaticMeshComponent (Utilities|Array|Get(acopy) (Variables|Default|GetButtons) (Variables|Default|GetCurrentNote))))
        (Rendering|Material|SetMaterial _asstatic_mesh_component_2 0 "/Game/Materials/M_COLORGreen__Inst.M_COLORGreen__Inst")
        (Math|Integer|IncrementInt (Variables|Default|GetNoteLoop))))
    (else
      (Utilities|Time|ClearandInvalidateTimerbyHandle (Variables|Default|GetPlayNoteTimer))
      (Variables|Default|SetIsinputMode true)
      (Variables|Default|SetNoteLoop 0))))

(fn UpdateGameLoop
  (Math|Integer|IncrementInt (Variables|Default|GetCurrentSequenceLoop)
    (:%20%20
      (CallFunction|CalculateNotes)
      (CallFunction|PlayNoteSequence))))

(fn TryPressButton
  (params (Object :type Actor%20Component%20Object%20Reference))
  (bind _asstatic_mesh_component (Utilities|Casting|CastToStaticMeshComponent Object)
    (:then
      (bind _output_get (LocalVariables|SetLocalButton _asstatic_mesh_component))
      (LocalVariables|SetLocalButtonID (Utilities|Array|FindItem (Variables|Default|GetButtons) _output_get))
      (if (== (Utilities|Array|FindItem (Variables|Default|GetButtons) _output_get) (Utilities|Array|Get(acopy) (Variables|Default|GetNotes) (Variables|Default|GetNoteLoop)))
        (Rendering|Material|SetMaterial (LocalVariables|GetLocalButton) 0 "/Game/Materials/M_Materials_Inst.M_Materials_Inst")
        (Math|Integer|IncrementInt (Variables|Default|GetNoteLoop)
          (:%20%20
            (if (>= (Variables|Default|GetNoteLoop) (Variables|Default|GetSizeOdSequence))
              (CallFunction|UpdateGameLoop))
            (return true true (LocalVariables|GetLocalButton) (LocalVariables|GetLocalButtonID))))
        (else
          (Rendering|Material|SetMaterial (LocalVariables|GetLocalButton) 0 "/Game/Materials/M_Materials_Inst_Inst.M_Materials_Inst_Inst")
          ;[1 1 1] ???
          (Variables|Default|SetCurrentSequenceLoop -1)
          (CallFunction|UpdateGameLoop)
          (return true false (LocalVariables|GetLocalButton) (LocalVariables|GetLocalButtonID)))))
    (:CastFailed
      (return false false 0 0))))

(fn InteractButton
  (params (Correct :type Boolean) (ButonID :type Integer))
  (Variables|Default|SetActiveButton ButonID)
  (Utilities|Time|SetTimerbyFunctionName 0 "ClearActiveButton" (Variables|Default|GetSpeedTime))
  (Audio|PlaySoundatLocation (Utilities|Array|Get(acopy) (Variables|Default|GetSounds) (Variables|Default|GetActiveButton)) (Transformation|GetWorldLocation (Variables|Default|Getmusic_games_Base)) "0, 0, 0" 1.0 1.0 0.0 0 0 0))

(fn ClearActiveButton
  (bind _asstatic_mesh_component (Utilities|Casting|CastToStaticMeshComponent (Utilities|Array|Get(acopy) (Variables|Default|GetButtons) (Variables|Default|GetActiveButton))))
  (Rendering|Material|SetMaterial _asstatic_mesh_component 0 "/Game/Materials/M_COLORGreen__Inst.M_COLORGreen__Inst"))