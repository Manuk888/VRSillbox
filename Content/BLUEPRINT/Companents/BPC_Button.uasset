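; BPC_Button is a component for a physical VR push button, pressed by either grab collision of BP_VRPawn.
; Overlap starts ticking, which moves the button along local Z with the hand within a clamped depth, then interpolates it back on release.
; Crossing the toggle depth updates state in momentary or toggle mode, with a minimum time between changes.
; State changes fire the ButtonPressed dispatcher and swap between green and steel materials.
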(event Custom|ComponentBeginOverlap
  (params (OverlappedComponent :type Primitive%20Component%20Object%20Reference) (OtherActor :type Actor%20Object%20Reference) (OtherComp :type Primitive%20Component%20Object%20Reference) (OtherBodyIndex :type Integer) (bFromSweep :type Boolean) (SweepResult :type Hit%20Result%20Structure%20%28by%20ref%29))
  (bind _asbp_vrpawn (Utilities|Casting|CastToBP_VRPawn OtherActor))
  (bind _output_get (Variables|Default|SetFocusActor _asbp_vrpawn))
  (if (or (== OtherComp (Variables|/Game/BLUEPRINT/Game/BP_VRPawn.BP_VRPawn_C|GetLeftGrapCollision _output_get)) (== OtherComp (Variables|/Game/BLUEPRINT/Game/BP_VRPawn.BP_VRPawn_C|GetRightGrapCollision _output_get)))
    (bind _output_get_2 (Variables|Default|SetFoucedComponent (select (== OtherComp (Variables|/Game/BLUEPRINT/Game/BP_VRPawn.BP_VRPawn_C|GetRightGrapCollision _output_get)) (Variables|/Game/BLUEPRINT/Game/BP_VRPawn.BP_VRPawn_C|GetRightGrapCollision _output_get) (Variables|/Game/BLUEPRINT/Game/BP_VRPawn.BP_VRPawn_C|GetLeftGrapCollision _output_get))))
    (CallFunction|StartButtonTransforming _output_get_2)))

(event Custom|ComponentEndOverlap
  (params (OverlappedComponent :type Primitive%20Component%20Object%20Reference) (OtherActor :type Actor%20Object%20Reference) (OtherComp :type Primitive%20Component%20Object%20Reference) (OtherBodyIndex :type Integer))
  (if (Variables|States|GetisEnablet)
    (if (== OtherActor (Variables|Default|GetFocusActor))
      (Variables|Default|SetFocusActor 0)
      (Variables|Default|SetFoucedComponent 0)
      (Variables|States|SetisEnablet false))))

(event EventBeginPlay
  (Collision|BindEventtoOnComponentBeginOverlap (EventDispatchers|CreateEvent :!event Custom|ComponentBeginOverlap))
  (Collision|BindEventtoOnComponentEndOverlap (EventDispatchers|CreateEvent :!event Custom|ComponentEndOverlap))
  (Variables|Transform|SetStartUpTransfotm (Transformation|GetRelativeTransform)))

(event EventTick
  (params (DeltaSeconds :type Float%20%28single-precision%29))
  (Utilities|FlowControl|Sequence
    (:then_0
      (if (Variables|States|GetisEnablet)
        (CallFunction|UpdateButtonLocation)
        (elif (not (Variables|States|GetLerping))
          (Variables|Default|SetFocusActor 0)
          (Variables|Default|SetFoucedComponent 0)
          (Variables|States|SetLerping true))))
    (:then_1
      (CallFunction|LerpReturnMovingButton)
      (CallFunction|UpdateButtonSateandColor))))

(fn StartButtonTransforming
  (params (Component :type Sphere%20Component%20Object%20Reference))
  (bind _currenttransform (CallFunction|GetCurrentTransform))
  (Variables|Transform|SetSturtUpLocal%20Z (.z (Math|Transform|InverseTransformLocation _currenttransform (Transformation|GetWorldLocation Component))))
  (Variables|Transform|SetStartUpComponent%20Z (.z (Math|Transform|InverseTransformLocation _currenttransform (Transformation|GetWorldLocation))))
  (Components|Tick|SetComponentTickEnabled true)
  (Variables|States|SetLerping false)
  (Variables|States|SetToggledThisTouch true)
  (Variables|States|SetisEnablet true))

(fn GetCurrentTransform
  (Variables|Default|GetFocusActor
    (:then
      (return (Math|Transform|ComposeTransforms (Variables|Transform|GetStartUpTransfotm) (Transformation|GetWorldTransform (Transformation|GetAttachParent)))))
    (:else
      (return (Variables|Transform|GetStartUpTransfotm)))))

(fn UpdateButtonLocation
  (bind _currenttransform (CallFunction|GetCurrentTransform))
  (bind _foucedcomponent (Variables|Default|GetFoucedComponent))
  (bind _sturtuplocal_z (Variables|Transform|GetSturtUpLocal%20Z))
  (bind _maxmovedistance (Variables|MainSettings|GetMaxMoveDistance))
  (bind _returnvalue (Transformation|GetWorldLocation _foucedcomponent))
  (bind _returnvalue_2 (Math|Transform|InverseTransformLocation _currenttransform _returnvalue))
  (bind _returnvalue_3 (- _sturtuplocal_z (.z _returnvalue_2)))
  (bind _returnvalue_4 (Math|Float|Clamp(Float) _returnvalue_3 0.0 _maxmovedistance))
  (if (> _returnvalue_4 0.0)
    (Transformation|SetRelativeLocation (Math|Transform|TransformLocation (Variables|Transform|GetStartUpTransfotm) (Math|Vector|MakeVector 0.0 0.0 (Math|Float|Clamp(Float) (+ (Variables|Transform|GetStartUpComponent%20Z) (* _returnvalue_4 -1.0)) (* (Variables|MainSettings|GetMaxMoveDistance) -1.0)))) false false)))

(fn LerpReturnMovingButton
  (bind _returnvalue (Utilities|Time|GetWorldDeltaSeconds))
  (bind _relativelocation (Variables|Default|GetRelativeLocation))
  (bind _startuptransfotm (Variables|Transform|GetStartUpTransfotm))
  (bind _returnspeed (Variables|MainSettings|GetReturnSpeed))
  (bind _returnvalue_2 (Math|Interpolation|VInterptoConstant _relativelocation (.location _startuptransfotm) _returnvalue _returnspeed))
  (if (Variables|States|GetLerping)
    (Transformation|SetRelativeLocation _returnvalue_2 false false)
    (if (Math|Vector|Equal(Vector) _returnvalue_2 "0, 0, 0" 0.0001)
      (Variables|States|SetLerping false)
      (Components|Tick|SetComponentTickEnabled false))))

(fn UpdateButtonSateandColor
  (bind _startuptransfotm (Variables|Transform|GetStartUpTransfotm))
  (bind _relativelocation (Variables|Default|GetRelativeLocation))
  (bind _togglingzoneheight (Variables|MainSettings|GetTogglingZoneHeight))
  (bind _returnvalue (Math|Transform|InverseTransformLocation _startuptransfotm _relativelocation))
  (bind _returnvalue_2 (* _togglingzoneheight -1.0))
  (bind _returnvalue_3 (+ _returnvalue_2 0.001))
  (bind _returnvalue_4 (<= (.z _returnvalue) _returnvalue_3))
  (if (Math|Boolean|NotEqual(Boolean) _returnvalue_4 (Variables|States|GetButtonState))
    (Utilities|FlowControl|DoOnce false :!label _label
      (:Completed
        (if (Variables|Default|GetTogglingButton)
          (if (Variables|States|GetToggledThisTouch)
            (bind _sucess (CallFunction|CheckButtonPresse (Variables|States|GetButtonState)))
            (CallFunction|SetButtonColor _sucess))
          (else
            (bind _output_get (Variables|States|SetButtonState _returnvalue_4))
            (CallFunction|CheckButtonPresse _output_get)
            (CallFunction|SetButtonColor _output_get)))))
    (else
      (goto _label Reset))))

(fn CheckButtonPresse
  (params (State :type Boolean))
  (if (>= (Math|Timespan|GetTotalSeconds (- (Math|DateTime|Now) (Variables|Default|GetLastToggleTime))) (Variables|MainSettings|GetMaxTimeBetweenToggle))
    (if (Variables|Default|GetTogglingButton)
      (if (Variables|States|GetToggledThisTouch)
        (Variables|Default|SetTogglingButton (not (Variables|States|GetToggledThisTouch)))
        (bind _output_get (Variables|States|SetButtonState (not (Variables|States|GetButtonState))))
        (Default|CallButtonPressed _output_get)
        (Variables|Default|SetLastToggleTime (Math|DateTime|Now))
        (return _output_get)
        (else
          (Variables|States|SetToggledThisTouch (not (Variables|States|GetToggledThisTouch)))))
      (else
        (bind _output_get_2 (Variables|States|SetButtonState State))
        (Default|CallButtonPressed _output_get_2)
        (Variables|Default|SetLastToggleTime (Math|DateTime|Now))))
    (else
      (return false))))

(fn SetButtonColor
  (params (State :type Boolean))
  (if State
    (Rendering|Material|SetMaterial 0 "/Game/Materials/M_COLORGreen__Inst.M_COLORGreen__Inst")
    (else
      (Rendering|Material|SetMaterial 0 "/Game/StarterContent/Materials/M_Metal_Steel.M_Metal_Steel"))))